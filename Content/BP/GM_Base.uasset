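; GM_Base is a game mode Blueprint that ramps up difficulty over time and ends the game at a target time.
; Each Tick, once TargetTimes has an index 2, it shrinks ReactionTime and InsultTime from their start values with elapsed time, clamped to minimums, and prints both on screen.
; When game time reaches that third target, GameOver pauses the game and shows the test end screen widget.
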(event Custom|GameOver
  (Game|SetGamePaused true)
  (bind _returnvalue (UserInterface|CreateWidget "/Game/UI/UI_TestEndScreenWidget.UI_TestEndScreenWidget_C"))
  (UserInterface|Viewport|AddtoViewport _returnvalue 0)
  (Development|PrintString "Hello"))

(event EventBeginPlay)

(event EventTick
  (params (DeltaSeconds :type Float%20%28single-precision%29))
  (if (Utilities|Array|IsValidIndex (Variables|Default|GetTargetTimes) 2)
    (Utilities|FlowControl|Sequence
      (:then_0
        (bind _output_get (Variables|Default|SetReactionTime (Math|Float|Max(Float) (- (Variables|Default|GetStartReactionTime) (/ (Utilities|Time|GetTimeSeconds) 3e+01)) (Variables|Default|GetMinReactionTime))))
        (Development|PrintString (Utilities|String|ToString(Float) _output_get) true false "(R=0.000000,G=0.660000,B=1.000000,A=1.000000)" 0.0)
        (bind _output_get_2 (Variables|Default|SetInsultTime (Math|Float|Max(Float) (- (Variables|Default|GetStartInsultTime) (/ (Utilities|Time|GetTimeSeconds) 3e+01)) (Variables|Default|GetMinInsultTime))))
        (Development|PrintString (Utilities|String|ToString(Float) _output_get_2) true false "(R=0.000000,G=0.660000,B=1.000000,A=1.000000)" 0.0))
      (:then_1
        (if (>= (Utilities|Time|GetTimeSeconds) (Utilities|Array|Get(acopy) (Variables|Default|GetTargetTimes) 2))
          (CallFunction|GameOver))))))

(fn ConstructionScript)