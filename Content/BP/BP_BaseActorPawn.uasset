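; Base pawn that walks to a target, then periodically prepares an insult that ends the game unless the player clicks it in time.
; Tick moves it horizontally toward TargetTransform and calls Activate on arrival, starting a random reaction delay from GM_Base.
; When that timer fires, SetInsultTimer shows the UI_InsultBar widget and schedules Insult, which calls GameOver.
; Clicking the skeletal mesh during preparation hides the bar, cancels that timer and restarts the delay.
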(event OnClicked(SkeletalMesh)
  (params (TouchedComponent :type Primitive%20Component%20Object%20Reference) (ButtonPressed :type Key%20Structure))
  (if (Variables|Default|GetisPreparingInsult)
    (Variables|Default|SetisPreparingInsult false)
    (Rendering|SetVisibility (Variables|Default|GetWidget) false false)
    (CallFunction|DelayInsultStart)
    (Utilities|Time|ClearandInvalidateTimerbyHandle (Variables|Default|GetInsult_TH))))

(event Custom|Activate
  (Variables|Default|SetisMoving false)
  (CallFunction|DelayInsultStart))

(event Custom|Insult
  (bind _asgm_base (Utilities|Casting|CastToGM_Base (Game|GetGameMode)))
  (Default|GameOver _asgm_base))

(event Custom|DelayInsultStart
  (bind _returnvalue (Game|GetGameMode))
  (bind _asgm_base (Utilities|Casting|CastToGM_Base _returnvalue))
  (bind _returnvalue_2 (Utilities|Time|SetTimerbyFunctionName 0 "SetInsultTimer" (Math|Random|RandomFloatinRange (Variables|/Game/BP/GM_Base.GM_Base_C|GetMinReactionTime _asgm_base) (Variables|/Game/BP/GM_Base.GM_Base_C|GetReactionTime _asgm_base))))
  (Variables|Default|SetSetInsultTimer_TH _returnvalue_2))

(event EventBeginPlay
  (Rendering|SetVisibility (Variables|Default|GetWidget) false false))

(event EventTick
  (params (DeltaSeconds :type Float%20%28single-precision%29))
  (bind _returnvalue (Transformation|GetActorLocation))
  (bind _targettransform (Variables|Default|GetTargetTransform))
  (bind (_x _y) (Math|Vector|BreakVector _returnvalue))
  (bind _location (Math|Transform|BreakTransform _targettransform))
  (bind (_x_2 _y_2) (Math|Vector|BreakVector _location))
  (if (Variables|Default|GetisMoving)
    (if (<= (Math|Vector|VectorLengthXY (- (.Location (Math|Transform|BreakTransform (Variables|Default|GetTargetTransform))) (Transformation|GetActorLocation))) 2e+01)
      (CallFunction|Activate)
      (else
        (Transformation|SetActorLocation (+ (Transformation|GetActorLocation) (* (Math|Vector|Normalize (Math|Vector|MakeVector (- _x_2 _x) (- _y_2 _y) 0.0)) (* (Variables|Default|GetSpeed) (Utilities|Time|GetWorldDeltaSeconds)))) false false)))))

(fn ConstructionScript)

(fn SetInsultTimer
  (bind _returnvalue (Game|GetGameMode))
  (bind _asgm_base (Utilities|Casting|CastToGM_Base _returnvalue))
  (Variables|Default|SetTime (Math|Random|RandomFloatinRange (Variables|/Game/BP/GM_Base.GM_Base_C|GetMinInsultTime _asgm_base) (Variables|/Game/BP/GM_Base.GM_Base_C|GetInsultTime _asgm_base)))
  (Rendering|SetVisibility (Variables|Default|GetWidget) true false)
  (bind _asui_insult_bar (Utilities|Casting|CastToUI_InsultBar (UserInterface|GetUserWidgetObject (Variables|Default|GetWidget))))
  (Default|Activate _asui_insult_bar (Variables|Default|GetTime))
  (bind _returnvalue_2 (Utilities|Time|SetTimerbyFunctionName 0 "Insult" (Variables|Default|GetTime)))
  (Variables|Default|SetInsult_TH _returnvalue_2)
  (Variables|Default|SetisPreparingInsult true))